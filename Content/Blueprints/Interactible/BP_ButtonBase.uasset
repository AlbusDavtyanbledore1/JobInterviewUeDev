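; BP_ButtonBase is an interactible button with a text label that triggers another object when used.
; It answers an interaction request by calling ResponceForInteractMessage on a valid instigator, passing itself.
; When interaction starts, it forwards StartInteraction to NestToActivate, if valid, with itself as instigator.
; The construction script shows ButtonNumberText on the TextRender, falling back to DefaultText when empty.
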(event EventRequesttoInteract
  (params (Instigator :type Actor%20Object%20Reference))
  (CallFunction|RequesttoInteractHandler Instigator))

(event EventStartInteraction
  (params (Instigator :type Actor%20Object%20Reference))
  (CallFunction|StartInteractionHandler Instigator))

(fn ConstructionScript
  (if (Utilities|Enum|NotEqual(Enum) (Variables|Settings|GetButtonNumberText) (LocalVariables|GetL_EmptyText))
    (Rendering|Components|TextRender|SetText (Variables|Default|GetTextRender) (Variables|Settings|GetButtonNumberText))
    (else
      (Rendering|Components|TextRender|SetText (Variables|Default|GetTextRender) (Variables|Default|GetDefaultText)))))

(fn RequesttoInteractHandler
  (params (Instigator :type Actor%20Object%20Reference))
  (LocalVariables|SetL_Instigator Instigator)
  (LocalVariables|GetL_Instigator
    (:then
      (Class|BPIInteraction|ResponceforInteract(Message) (LocalVariables|GetL_Instigator) self))
    (:else)))

(fn StartInteractionHandler
  (params (Instigator :type Actor%20Object%20Reference))
  (Utilities|IsValid (Variables|References|GetNestToActivate)
    (:Is%20Valid
      (Default|StartInteraction (Variables|References|GetNestToActivate) self))))