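; Base interactible turtle nest that spawns a single turtle when interacted with and shows a nest number on a text render.
; StartInteraction spawns the configured turtle class at SpawnPoint, assigns its AI controller class and blocks further spawns.
; Relative spawn and destination transforms become world transforms through runtime-added scene components.
; The destination component is created in the construction script and exposed through GetAiDestinationTransform.
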(event EventStartInteraction
  (params (Instigator :type Actor%20Object%20Reference))
  (CallFunction|StartInteractionHandler Instigator))

(fn ConstructionScript
  (Utilities|FlowControl|Sequence
    (:then_0
      ;[1 1 1] Construct nest number text
      (if (Utilities|Enum|NotEqual(Enum) (Variables|Settings|GetNestNumberText) (LocalVariables|GetL_EmptyText))
        (Rendering|Components|TextRender|SetText (Variables|Default|GetTextRender) (Variables|Settings|GetNestNumberText))
        (else
          (Rendering|Components|TextRender|SetText (Variables|Default|GetTextRender) (Variables|Default|GetDefaultNumberText)))))
    (:then_1
      ;[1 1 1] Construct destination point scene component for getting world location
      (bind _returnvalue (AddComponent|AddSceneComponent false (Variables|Settings|GetDestinationPoint)))
      (Variables|Default|SetDestinationLocalPoint _returnvalue))))

(fn StartInteractionHandler
  (params (Instigator :type Actor%20Object%20Reference))
  (if (and (!= (Variables|Settings|GetTurtleClass) 0) (not (Variables|Default|GetTurtleSpawned)))
    (Utilities|FlowControl|Sequence
      (:then_0
        ;[1 1 1] get world transform from relative spawn point
        (bind _returnvalue (AddComponent|AddSceneComponent false (Variables|Settings|GetSpawnPoint)))
        (bind _output_get (Variables|Default|SetSpawnLocalPoint _returnvalue))
        (LocalVariables|SetL_SpawnWorldTransform (Transformation|GetWorldTransform _output_get)))
      (:then_1
        ;[1 1 1] spawn ans set up turtle at world transform
        (bind _returnvalue_2 (Game|SpawnActorfromClass (Variables|Settings|GetTurtleClass) (LocalVariables|GetL_SpawnWorldTransform) "Undefined" 0 (Variables|Settings|GetTurtleAIController) 0))
        (bind _output_get_2 (Variables|References|SetTurtleReference _returnvalue_2))
        (Variables|/Script/Engine.Pawn|SetAIControllerClass _output_get_2 (Variables|Settings|GetTurtleAIController)))
      (:then_2
        (Variables|Default|SetTurtleSpawned true)))))

(fn GetAiDestinationTransform
  (return (Transformation|GetWorldTransform (Variables|Default|GetDestinationLocalPoint))))